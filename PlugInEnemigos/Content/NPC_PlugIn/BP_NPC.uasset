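; BP_NPC is a data-driven NPC character whose movement and AI come from its NPCData.
; On BeginPlay, SetVariables applies the data's velocity as max walk speed, then casts the controller to AI_NPC.
; It runs the aggressive, friendly or neutral behavior tree according to NPCBehaviour.
; The Roaming flag is then written to the blackboard, though the key name shown is the literal "None".
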(event `self.ReceiveBeginPlay`
  (`self.Set Variables`))

(fn `Set Variables`
  (set `CharacterMovementComponent.MaxWalkSpeed` (`/Game/NPC_PlugIn/Asset_Data/PAD_NPC_Variables.Velocity` (`self.NPC Data`)) (`self.CharacterMovement`))
  (bind _asai_npc (cast `/Game/NPC_PlugIn/AI_NPC` (`self.GetController`)))
  (switch `/Game/NPC_PlugIn/Asset_Data/Variables_AssetData/TypeOfBehabiour` (`/Game/NPC_PlugIn/Asset_Data/PAD_NPC_Variables.NPC Behaviour` (`self.NPC Data`))
    (:`NewEnumerator0`
      (`AIController.RunBehaviorTree` _asai_npc "/Game/NPC_PlugIn/BehabiourTrees/BT_NPC_Agresivo.BT_NPC_Agresivo"))
    (:`NewEnumerator1`
      (`AIController.RunBehaviorTree` _asai_npc "/Game/NPC_PlugIn/BehabiourTrees/BT_NPC_Amigable.BT_NPC_Amigable"))
    (:`NewEnumerator2`
      (`AIController.RunBehaviorTree` _asai_npc "/Game/NPC_PlugIn/BehabiourTrees/BT_NPC_Neutral.BT_NPC_Neutral")))
  (`BlackboardComponent.SetValueAsBool` (`AIBlueprintHelperLibrary.GetBlackboard` null) "None" (`/Game/NPC_PlugIn/Asset_Data/PAD_NPC_Variables.Roaming` (`self.NPC Data`))))

(fn `UserConstructionScript`)